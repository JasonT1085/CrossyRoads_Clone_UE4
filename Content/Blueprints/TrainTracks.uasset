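; Train track lane actor that spawns moving trains and awards the player score on first contact with its mesh.
; On BeginPlay it randomly picks one side and starts a looping timer with a randomized interval, both fixed thereafter.
; Each tick of that timer spawns a Train, negating its projectile velocity for left-side spawns.
; Two trigger zones destroy overlapping trains, while a DoOnce limits the BP_Player score award to one.
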(event `self.ReceiveBeginPlay`
  (set `self.SpawnLocation` (`SceneComponent.K2_GetComponentLocation` (`self.SpawnPoint`)))
  (set `self.SpawnLocationLeft` (`SceneComponent.K2_GetComponentLocation` (`self.SpawnpointLeft`)))
  (set `self.SetStartLocation` (`KismetMathLibrary.RandomBool`))
  (`KismetSystemLibrary.K2_SetTimerDelegate` (delegate `Spawn Logs`) (`KismetMathLibrary.RandomFloatInRange` 5.0 7.0) true))

(event `Spawn Logs`
  (if (`self.SetStartLocation`)
    (`|SpawnActorFromClass` "/Game/Blueprints/Train.Train_C" (`KismetMathLibrary.MakeTransform` (`self.SpawnLocation`)) "Undefined" "OverrideRootScale" null null)
    (else
      (bind _returnvalue (`|SpawnActorFromClass` "/Game/Blueprints/Train.Train_C" (`KismetMathLibrary.MakeTransform` (`self.SpawnLocationLeft`)) "Undefined" "OverrideRootScale" null null))
      (bind _projectilemovement (`/Game/Blueprints/Train.ProjectileMovement` _returnvalue))
      (set `MovementComponent.Velocity` (`KismetMathLibrary.NegateVector` (`MovementComponent.Velocity` _projectilemovement)) _projectilemovement))))

(event `self.TriggerZone.OnComponentBeginOverlap`
  (params (OverlappedComponent :type "PrimitiveComponent Object Reference") (OtherActor :type "Actor Object Reference") (OtherComp :type "PrimitiveComponent Object Reference") (OtherBodyIndex :type Integer) (bFromSweep :type Boolean) (SweepResult :type "HitResult Structure (by ref)"))
  (bind _astrain (cast `/Game/Blueprints/Train` OtherActor))
  (`self.K2_DestroyActor` _astrain))

(event `self.TriggerZone1.OnComponentBeginOverlap`
  (params (OverlappedComponent :type "PrimitiveComponent Object Reference") (OtherActor :type "Actor Object Reference") (OtherComp :type "PrimitiveComponent Object Reference") (OtherBodyIndex :type Integer) (bFromSweep :type Boolean) (SweepResult :type "HitResult Structure (by ref)"))
  (bind _astrain (cast `/Game/Blueprints/Train` OtherActor))
  (`self.K2_DestroyActor` _astrain))

(event `self.StaticMesh.OnComponentHit`
  (params (HitComponent :type "PrimitiveComponent Object Reference") (OtherActor :type "Actor Object Reference") (OtherComp :type "PrimitiveComponent Object Reference") (NormalImpulse :type "Vector Structure") (Hit :type "HitResult Structure (by ref)"))
  (bind _asbp_player (cast `/Game/Blueprints/BP_Player` OtherActor))
  (`/Engine/EditorBlueprintResources/StandardMacros.DoOnce` false
    (:`Completed`
      (`/Game/Blueprints/BP_Player.Add Score` _asbp_player))))

(fn `UserConstructionScript`)