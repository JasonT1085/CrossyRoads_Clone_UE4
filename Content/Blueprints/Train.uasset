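; Train hazard actor that flattens the player on contact and has a level-restart event for player death.
; On BeginPlay a random roll can swap its mesh, though the 0–1 range never reaches the Train4 case.
; Box overlap with BP_Player disables input, squashes and lowers the player's mesh, plays a hurt sound and spawns an eagle at the player's EagleSpawn point.
; OnPlayerDeath reopens the current level.
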(event `self.ReceiveBeginPlay`
  (bind _staticmesh (`self.StaticMesh`))
  (switch `int` (`KismetMathLibrary.RandomIntegerInRange` 0 1)
    (:`1`
      (`StaticMeshComponent.SetStaticMesh` _staticmesh "/Game/crossy_road_meshes_fbx/train2.train2"))
    (:`2`
      (`StaticMeshComponent.SetStaticMesh` _staticmesh "/Game/crossy_road_meshes_fbx/train4.train4"))))

(event `self.Box.OnComponentBeginOverlap`
  (params (OverlappedComponent :type "PrimitiveComponent Object Reference") (OtherActor :type "Actor Object Reference") (OtherComp :type "PrimitiveComponent Object Reference") (OtherBodyIndex :type Integer) (bFromSweep :type Boolean) (SweepResult :type "HitResult Structure (by ref)"))
  (bind _asbp_player (cast `/Game/Blueprints/BP_Player` OtherActor))
  (`self.DisableInput` _asbp_player null)
  (bind _staticmesh (`/Game/Blueprints/BP_Player.StaticMesh` _asbp_player))
  (bind (_relativescale3d_x _relativescale3d_y) (`KismetMathLibrary.BreakVector` (`SceneComponent.RelativeScale3D` _staticmesh)))
  (`SceneComponent.SetRelativeScale3D` _staticmesh (`KismetMathLibrary.MakeVector` _relativescale3d_x _relativescale3d_y))
  (bind (_relativelocation_x _relativelocation_y) (`KismetMathLibrary.BreakVector` (`SceneComponent.RelativeLocation` _staticmesh)))
  (`SceneComponent.K2_SetRelativeLocation` _staticmesh (`KismetMathLibrary.MakeVector` _relativelocation_x _relativelocation_y -40.0) false false)
  (`GameplayStatics.PlaySound2D` "/Game/Sound/Chicken_hurt1.Chicken_hurt1" 1.0 1.0 0.0 null null)
  (`|SpawnActorFromClass` "/Game/Blueprints/BP_Eagle.BP_Eagle_C" (`KismetMathLibrary.MakeTransform` (`SceneComponent.K2_GetComponentLocation` (`/Game/Blueprints/BP_Player.EagleSpawn` _asbp_player))) "Undefined" "OverrideRootScale" null null))

(event `OnPlayerDeath`
  (bind _returnvalue (`GameplayStatics.GetCurrentLevelName` true))
  (`GameplayStatics.OpenLevel` (`KismetStringLibrary.Conv_StringToName` _returnvalue)))

(fn `UserConstructionScript`)