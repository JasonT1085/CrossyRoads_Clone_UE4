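; BP_Eagle is an eagle hazard that kills the player on contact and restarts the level.
; It plays a 2D eagle sound on BeginPlay.
; When its Box overlaps BP_Player, it hides the player by scaling their StaticMesh to zero, waits briefly, then calls OnPlayerDeath, which reopens the current level by name.
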(event `self.ReceiveBeginPlay`
  (`GameplayStatics.PlaySound2D` "/Game/Sound/eagle.eagle" 1.0 1.0 0.0 null null))

(event `self.Box.OnComponentBeginOverlap`
  (params (OverlappedComponent :type "PrimitiveComponent Object Reference") (OtherActor :type "Actor Object Reference") (OtherComp :type "PrimitiveComponent Object Reference") (OtherBodyIndex :type Integer) (bFromSweep :type Boolean) (SweepResult :type "HitResult Structure (by ref)"))
  (bind _asbp_player (cast `/Game/Blueprints/BP_Player` OtherActor))
  (`SceneComponent.SetRelativeScale3D` (`/Game/Blueprints/BP_Player.StaticMesh` _asbp_player) (0.0 0.0 0.0))
  (`KismetSystemLibrary.Delay` 3.0)
  (`self.OnPlayerDeath`))

(event `OnPlayerDeath`
  (bind _returnvalue (`GameplayStatics.GetCurrentLevelName` true))
  (`GameplayStatics.OpenLevel` (`KismetStringLibrary.Conv_StringToName` _returnvalue)))

(fn `UserConstructionScript`)