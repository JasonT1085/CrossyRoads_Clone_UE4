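; Grass lane actor that decorates itself with obstacles and a coin, and awards score when the player hits it.
; BeginPlay randomly applies a dark grass mesh, then steps along Y over the Start-to-End distance, occasionally spawning TreeRockSpawner actors.
; A DoOnce flag lets the first successful roll spawn a BP_Coin instead.
; The mesh's hit event calls AddScore on BP_Player through a DoOnce gate, so each lane scores only once.
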(event `self.ReceiveBeginPlay`
  (bind (_startlocation_x _startlocation_y _startlocation_z) (`KismetMathLibrary.BreakVector` (`self.StartLocation`)))
  (`|ExecutionSequence`
    (:`then_0`
      (switch `int` (`KismetMathLibrary.RandomIntegerInRange` 0 2)
        (:`0`
          (`StaticMeshComponent.SetStaticMesh` (`self.StaticMesh`) "/Game/crossy_road_meshes_fbx/1lane_grass_dark.1lane_grass_dark"))))
    (:`then_1`
      (set `self.StartLocation` (`SceneComponent.K2_GetComponentLocation` (`self.start`)))
      (set `self.EndLocation` (`SceneComponent.K2_GetComponentLocation` (`self.end`)))
      (for _index (range (+ (`KismetMathLibrary.FTrunc` (/ (`KismetMathLibrary.Vector_Distance` (`self.StartLocation`) (`self.EndLocation`)) 85.0)) 1))
        (if (> (`KismetMathLibrary.RandomFloat`) 0.9)
          (if (`self.doOnce`)
            (bind _returnvalue (`KismetMathLibrary.MakeVector` _startlocation_x (+ (`KismetMathLibrary.Conv_IntToDouble` (* _index 90)) (.y (`self.StartLocation`))) _startlocation_z))
            (`|SpawnActorFromClass` "/Game/Blueprints/BP_Coin.BP_Coin_C" (`KismetMathLibrary.MakeTransform` _returnvalue) "Undefined" "OverrideRootScale" null null)
            (set `self.doOnce` false)
            (else
              (`|SpawnActorFromClass` "/Game/Blueprints/TreeRockSpawner.TreeRockSpawner_C" (`KismetMathLibrary.MakeTransform` _returnvalue) "Undefined" "OverrideRootScale" null null))))))))

(event `self.StaticMesh.OnComponentHit`
  (params (HitComponent :type "PrimitiveComponent Object Reference") (OtherActor :type "Actor Object Reference") (OtherComp :type "PrimitiveComponent Object Reference") (NormalImpulse :type "Vector Structure") (Hit :type "HitResult Structure (by ref)"))
  (bind _asbp_player (cast `/Game/Blueprints/BP_Player` OtherActor))
  (`/Engine/EditorBlueprintResources/StandardMacros.DoOnce` false
    (:`Completed`
      (`/Game/Blueprints/BP_Player.Add Score` _asbp_player))))

(fn `UserConstructionScript`)