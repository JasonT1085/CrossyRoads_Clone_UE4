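; VehicleLaneSpawner is a lane terrain actor that sends vehicles across it and awards score when the player first hits its mesh.
; On BeginPlay it creates a VehicleSpawner linked back to itself, randomly picks one of two spawn points, and requests vehicles there on a looping timer with a once-randomized interval.
; Two trigger zones destroy overlapping VehiclesLeft actors, and a DoOnce limits BP_Player scoring to once per lane.
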(event `self.ReceiveBeginPlay`
  (set `self.SpawnLocation` (`SceneComponent.K2_GetComponentLocation` (`self.SpawnPoint`)))
  (set `self.SpawnLocationLeft` (`SceneComponent.K2_GetComponentLocation` (`self.SpawnpointLeft`)))
  (bind _returnvalue (`|SpawnActorFromClass` "/Game/Blueprints/VehicleSpawner.VehicleSpawner_C" (`KismetMathLibrary.MakeTransform` (0.0 0.0 0.0)) "Undefined" "OverrideRootScale" null null))
  (bind _output_get (set `self.VehicleSpawner` _returnvalue))
  (set `/Game/Blueprints/VehicleSpawner.BP_Terrain` self _output_get)
  (set `self.SetStartLocation` (`KismetMathLibrary.RandomBool`))
  (`KismetSystemLibrary.K2_SetTimerDelegate` (delegate `Spawn Vehicle`) (`KismetMathLibrary.RandomFloatInRange` 2.0 3.0) true))

(event `Spawn Vehicle`
  (if (`self.SetStartLocation`)
    (`/Game/Blueprints/VehicleSpawner.SpawnVehicle` (stale `self.ReceiveBeginPlay` _output_get) (`self.SpawnLocation`))
    (else
      (`/Game/Blueprints/VehicleSpawner.SpawnVehicle` (stale `self.ReceiveBeginPlay` _output_get) (`self.SpawnLocationLeft`)))))

(event `self.TriggerZone.OnComponentBeginOverlap`
  (params (OverlappedComponent :type "PrimitiveComponent Object Reference") (OtherActor :type "Actor Object Reference") (OtherComp :type "PrimitiveComponent Object Reference") (OtherBodyIndex :type Integer) (bFromSweep :type Boolean) (SweepResult :type "HitResult Structure (by ref)"))
  (bind _asvehicles_left (cast `/Game/Blueprints/VehiclesLeft` OtherActor))
  (`self.K2_DestroyActor` _asvehicles_left))

(event `self.StaticMesh.OnComponentHit`
  (params (HitComponent :type "PrimitiveComponent Object Reference") (OtherActor :type "Actor Object Reference") (OtherComp :type "PrimitiveComponent Object Reference") (NormalImpulse :type "Vector Structure") (Hit :type "HitResult Structure (by ref)"))
  (bind _asbp_player (cast `/Game/Blueprints/BP_Player` OtherActor))
  (`/Engine/EditorBlueprintResources/StandardMacros.DoOnce` false
    (:`Completed`
      (`/Game/Blueprints/BP_Player.Add Score` _asbp_player))))

(event `self.TriggerZone1.OnComponentBeginOverlap`
  (params (OverlappedComponent :type "PrimitiveComponent Object Reference") (OtherActor :type "Actor Object Reference") (OtherComp :type "PrimitiveComponent Object Reference") (OtherBodyIndex :type Integer) (bFromSweep :type Boolean) (SweepResult :type "HitResult Structure (by ref)"))
  (bind _asvehicles_left (cast `/Game/Blueprints/VehiclesLeft` OtherActor))
  (`self.K2_DestroyActor` _asvehicles_left))

(fn `UserConstructionScript`)