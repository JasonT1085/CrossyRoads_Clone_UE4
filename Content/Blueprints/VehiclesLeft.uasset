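; Vehicle hazard that runs over BP_Player and restarts the current level.
; BeginPlay randomly picks one of four car meshes with a matching projectile movement speed; the Fedex variant also adjusts mesh height and box scale.
; Actor and mesh overlaps both flatten the player, disable its collision and reload after a delay.
; Only the actor path disables input and plays a hurt sound; only the mesh path destroys the player.
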(event `self.ReceiveBeginPlay`
  (bind _box (`self.Box`))
  (bind _projectilemovement (`self.ProjectileMovement`))
  (bind _projectilemovement_2 (`self.ProjectileMovement`))
  (bind _projectilemovement_3 (`self.ProjectileMovement`))
  (bind _projectilemovement_4 (`self.ProjectileMovement`))
  (bind (_relativescale3d_x _relativescale3d_y _relativescale3d_z) (`KismetMathLibrary.BreakVector` (`SceneComponent.RelativeScale3D` _box)))
  (bind (_relativelocation_x _relativelocation_y) (`KismetMathLibrary.BreakVector` (`SceneComponent.RelativeLocation` (`self.StaticMesh`))))
  (switch `int` (`KismetMathLibrary.RandomIntegerInRange` 0 3)
    (:`0`
      (`StaticMeshComponent.SetStaticMesh` (`self.StaticMesh`) "/Game/crossy_road_meshes_fbx/red_car.red_car")
      (set `ProjectileMovementComponent.InitialSpeed` 300.0 _projectilemovement_2)
      (set `ProjectileMovementComponent.MaxSpeed` 300.0 _projectilemovement_2)
      (`KismetSystemLibrary.Delay` 14.0))
    (:`1`
      (`StaticMeshComponent.SetStaticMesh` (`self.StaticMesh`) "/Game/crossy_road_meshes_fbx/fedex.fedex")
      (`SceneComponent.K2_SetRelativeLocation` (`self.StaticMesh`) (`KismetMathLibrary.MakeVector` _relativelocation_x _relativelocation_y 30.0) false false)
      (set `ProjectileMovementComponent.InitialSpeed` 250.0 _projectilemovement_3)
      (set `ProjectileMovementComponent.MaxSpeed` 250.0 _projectilemovement_3)
      (`SceneComponent.SetRelativeScale3D` _box (`KismetMathLibrary.MakeVector` _relativescale3d_x 4.0 _relativescale3d_z)))
    (:`2`
      (`StaticMeshComponent.SetStaticMesh` (`self.StaticMesh`) "/Game/crossy_road_meshes_fbx/police_car.police_car")
      (set `ProjectileMovementComponent.InitialSpeed` 400.0 _projectilemovement_4)
      (set `ProjectileMovementComponent.MaxSpeed` 400.0 _projectilemovement_4))
    (:`3`
      (`StaticMeshComponent.SetStaticMesh` (`self.StaticMesh`) "/Game/crossy_road_meshes_fbx/yellow_short_car.yellow_short_car")
      (set `ProjectileMovementComponent.InitialSpeed` 350.0 _projectilemovement)
      (set `ProjectileMovementComponent.MaxSpeed` 350.0 _projectilemovement))))

(event `self.ReceiveActorBeginOverlap`
  (params (OtherActor :type "Actor Object Reference"))
  (bind _asbp_player (cast `/Game/Blueprints/BP_Player` OtherActor))
  (`self.DisableInput` _asbp_player null)
  (bind _staticmesh (`/Game/Blueprints/BP_Player.StaticMesh` _asbp_player))
  (bind (_relativescale3d_x _relativescale3d_y) (`KismetMathLibrary.BreakVector` (`SceneComponent.RelativeScale3D` _staticmesh)))
  (`SceneComponent.SetRelativeScale3D` _staticmesh (`KismetMathLibrary.MakeVector` _relativescale3d_x _relativescale3d_y))
  (bind (_relativelocation_x _relativelocation_y) (`KismetMathLibrary.BreakVector` (`SceneComponent.RelativeLocation` _staticmesh)))
  (`SceneComponent.K2_SetRelativeLocation` _staticmesh (`KismetMathLibrary.MakeVector` _relativelocation_x _relativelocation_y -40.0) false false)
  (`PrimitiveComponent.SetCollisionEnabled` _staticmesh "NoCollision")
  (`PrimitiveComponent.SetCollisionEnabled` (`Character.CapsuleComponent` _asbp_player) "NoCollision")
  (`GameplayStatics.PlaySound2D` "/Game/Sound/Chicken_hurt1.Chicken_hurt1" 1.0 1.0 0.0 null null)
  (`KismetSystemLibrary.Delay` 3.0)
  (`/Engine/EditorBlueprintResources/StandardMacros.DoOnce` false
    (:`Completed`
      (`self.OnPlayerDeath`))))

(event `OnPlayerDeath`
  (bind _returnvalue (`GameplayStatics.GetCurrentLevelName` true))
  (`GameplayStatics.OpenLevel` (`KismetStringLibrary.Conv_StringToName` _returnvalue)))

(event `self.StaticMesh.OnComponentBeginOverlap`
  (params (OverlappedComponent :type "PrimitiveComponent Object Reference") (OtherActor :type "Actor Object Reference") (OtherComp :type "PrimitiveComponent Object Reference") (OtherBodyIndex :type Integer) (bFromSweep :type Boolean) (SweepResult :type "HitResult Structure (by ref)"))
  (bind _asbp_player (cast `/Game/Blueprints/BP_Player` OtherActor))
  (bind _staticmesh (`/Game/Blueprints/BP_Player.StaticMesh` _asbp_player))
  (bind (_relativescale3d_x _relativescale3d_y) (`KismetMathLibrary.BreakVector` (`SceneComponent.RelativeScale3D` _staticmesh)))
  (`SceneComponent.SetRelativeScale3D` _staticmesh (`KismetMathLibrary.MakeVector` _relativescale3d_x _relativescale3d_y))
  (bind (_relativelocation_x _relativelocation_y) (`KismetMathLibrary.BreakVector` (`SceneComponent.RelativeLocation` _staticmesh)))
  (`SceneComponent.K2_SetRelativeLocation` _staticmesh (`KismetMathLibrary.MakeVector` _relativelocation_x _relativelocation_y -40.0) false false)
  (`PrimitiveComponent.SetCollisionEnabled` _staticmesh "NoCollision")
  (`PrimitiveComponent.SetCollisionEnabled` (`Character.CapsuleComponent` _asbp_player) "NoCollision")
  (`KismetSystemLibrary.Delay` 3.0)
  (`self.K2_DestroyActor` _asbp_player)
  (`self.OnPlayerDeath`))

(fn `UserConstructionScript`)