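; Water lane actor that clears logs, kills the player in its hazard zones and awards score, despite its spawner name containing no spawn logic.
; Two trigger zones destroy overlapping Logs, and a score volume calls AddScore on BP_Player once.
; Two death zones and a drown volume disable input, shrink the player mesh to zero, then, once per volume, play hurt and splash sounds and reload the level after a delay.
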(event `self.ReceiveBeginPlay`)

(event `self.ReceiveTick`
  (params (DeltaSeconds :type "Float (single-precision)")))

(event `self.TriggerZone.OnComponentBeginOverlap`
  (params (OverlappedComponent :type "PrimitiveComponent Object Reference") (OtherActor :type "Actor Object Reference") (OtherComp :type "PrimitiveComponent Object Reference") (OtherBodyIndex :type Integer) (bFromSweep :type Boolean) (SweepResult :type "HitResult Structure (by ref)"))
  (bind _aslogs (cast `/Game/Blueprints/Logs` OtherActor))
  (`self.K2_DestroyActor` _aslogs))

(event `self.TriggerZone1.OnComponentBeginOverlap`
  (params (OverlappedComponent :type "PrimitiveComponent Object Reference") (OtherActor :type "Actor Object Reference") (OtherComp :type "PrimitiveComponent Object Reference") (OtherBodyIndex :type Integer) (bFromSweep :type Boolean) (SweepResult :type "HitResult Structure (by ref)"))
  (bind _aslogs (cast `/Game/Blueprints/Logs` OtherActor))
  (`self.K2_DestroyActor` _aslogs))

(event `OnPlayerDeath`
  (bind _returnvalue (`GameplayStatics.GetCurrentLevelName` true))
  (`GameplayStatics.OpenLevel` (`KismetStringLibrary.Conv_StringToName` _returnvalue)))

(event `self.DeathZone.OnComponentBeginOverlap`
  (params (OverlappedComponent :type "PrimitiveComponent Object Reference") (OtherActor :type "Actor Object Reference") (OtherComp :type "PrimitiveComponent Object Reference") (OtherBodyIndex :type Integer) (bFromSweep :type Boolean) (SweepResult :type "HitResult Structure (by ref)"))
  (bind _asbp_player (cast `/Game/Blueprints/BP_Player` OtherActor))
  (`self.DisableInput` _asbp_player null)
  (`SceneComponent.SetRelativeScale3D` (`/Game/Blueprints/BP_Player.StaticMesh` _asbp_player) (0.0 0.0 0.0))
  (`/Engine/EditorBlueprintResources/StandardMacros.DoOnce` false
    (:`Completed`
      (`GameplayStatics.PlaySound2D` "/Game/Sound/Chicken_hurt1.Chicken_hurt1" 1.0 1.0 0.0 null null)
      (`GameplayStatics.PlaySound2D` "/Game/Sound/352098__inspectorj__splash-jumping-d.352098__inspectorj__splash-jumping-d" 1.0 1.0 0.0 null null)
      (`KismetSystemLibrary.Delay` 2.0)
      (`self.OnPlayerDeath`))))

(event `self.DeathZone1.OnComponentBeginOverlap`
  (params (OverlappedComponent :type "PrimitiveComponent Object Reference") (OtherActor :type "Actor Object Reference") (OtherComp :type "PrimitiveComponent Object Reference") (OtherBodyIndex :type Integer) (bFromSweep :type Boolean) (SweepResult :type "HitResult Structure (by ref)"))
  (bind _asbp_player (cast `/Game/Blueprints/BP_Player` OtherActor))
  (`self.DisableInput` _asbp_player null)
  (`SceneComponent.SetRelativeScale3D` (`/Game/Blueprints/BP_Player.StaticMesh` _asbp_player) (0.0 0.0 0.0))
  (`/Engine/EditorBlueprintResources/StandardMacros.DoOnce` false
    (:`Completed`
      (`GameplayStatics.PlaySound2D` "/Game/Sound/Chicken_hurt1.Chicken_hurt1" 1.0 1.0 0.0 null null)
      (`GameplayStatics.PlaySound2D` "/Game/Sound/352098__inspectorj__splash-jumping-d.352098__inspectorj__splash-jumping-d" 1.0 1.0 0.0 null null)
      (`KismetSystemLibrary.Delay` 2.0)
      (`self.OnPlayerDeath`))))

(event `self.DrownCollision.OnComponentBeginOverlap`
  (params (OverlappedComponent :type "PrimitiveComponent Object Reference") (OtherActor :type "Actor Object Reference") (OtherComp :type "PrimitiveComponent Object Reference") (OtherBodyIndex :type Integer) (bFromSweep :type Boolean) (SweepResult :type "HitResult Structure (by ref)"))
  (bind _asbp_player (cast `/Game/Blueprints/BP_Player` OtherActor))
  (`self.DisableInput` _asbp_player null)
  (`SceneComponent.SetRelativeScale3D` (`/Game/Blueprints/BP_Player.StaticMesh` _asbp_player) (0.0 0.0 0.0))
  (`/Engine/EditorBlueprintResources/StandardMacros.DoOnce` false
    (:`Completed`
      (`GameplayStatics.PlaySound2D` "/Game/Sound/Chicken_hurt1.Chicken_hurt1" 1.0 1.0 0.0 null null)
      (`GameplayStatics.PlaySound2D` "/Game/Sound/352098__inspectorj__splash-jumping-d.352098__inspectorj__splash-jumping-d" 1.0 1.0 0.0 null null)
      (`KismetSystemLibrary.Delay` 2.0)
      (`self.OnPlayerDeath`))))

(event `self.ScoreCollision.OnComponentBeginOverlap`
  (params (OverlappedComponent :type "PrimitiveComponent Object Reference") (OtherActor :type "Actor Object Reference") (OtherComp :type "PrimitiveComponent Object Reference") (OtherBodyIndex :type Integer) (bFromSweep :type Boolean) (SweepResult :type "HitResult Structure (by ref)"))
  (bind _asbp_player (cast `/Game/Blueprints/BP_Player` OtherActor))
  (`/Engine/EditorBlueprintResources/StandardMacros.DoOnce` false
    (:`Completed`
      (`/Game/Blueprints/BP_Player.Add Score` _asbp_player))))

(fn `UserConstructionScript`)