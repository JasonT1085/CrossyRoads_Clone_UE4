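; Spawner that creates moving vehicles of the VehiclesLeft class for a BPTerrain piece and registers itself on each one.
; The terrain's SetStartLocation flag picks the travel direction, with the opposite direction reusing the class by rotating it 180 degrees and negating its projectile velocity.
; The initial spawn uses the terrain's SpawnPoint if a vehicle already exists, otherwise randomly one of two supplied locations.
; Logic that destroys all vehicles is present but never runs.
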(event `self.ReceiveBeginPlay`)

(fn `Spawn Initial Vehicles`
  (params (RightToLeft :type "Vector Structure") (LeftToRIght :type "Vector Structure"))
  (set `self.Left to Right` LeftToRIght)
  (set `self.RightToLeft` RightToLeft)
  (`/Engine/EditorBlueprintResources/StandardMacros.IsValid` (`self.Vehicle`)
    (:`Is Valid`
      (`self.SpawnVehicleAtSpawnPoint`))
    (:`Is Not Valid`
      (if (`KismetMathLibrary.RandomBool`)
        (`self.SpawnVehicle` (`self.RightToLeft`))
        (else
          (`self.SpawnVehicle` (`self.Left to Right`)))))))

(fn `SpawnVehicle`
  (params (SpawnLocation :type "Vector Structure"))
  (if (`/Game/Blueprints/VehicleLaneSpawner.SetStartLocation` (`self.BP_Terrain`))
    (bind _returnvalue (`|SpawnActorFromClass` "/Game/Blueprints/VehiclesLeft.VehiclesLeft_C" (`KismetMathLibrary.MakeTransform` SpawnLocation) "Undefined" "OverrideRootScale" null null))
    (bind _output_get (set `self.Vehicle` _returnvalue))
    (set `/Game/Blueprints/VehiclesLeft.VehicleSpawner` self _output_get)
    (else
      (bind _returnvalue_2 (`|SpawnActorFromClass` "/Game/Blueprints/VehiclesLeft.VehiclesLeft_C" (`KismetMathLibrary.MakeTransform` SpawnLocation (struct :`Yaw` 180.0)) "Undefined" "OverrideRootScale" null null))
      (bind _output_get_2 (set `self.Vehicle` _returnvalue_2))
      (bind _projectilemovement (`/Game/Blueprints/VehiclesLeft.ProjectileMovement` _output_get_2))
      (set `MovementComponent.Velocity` (`KismetMathLibrary.NegateVector` (`MovementComponent.Velocity` _projectilemovement)) _projectilemovement)
      (set `/Game/Blueprints/VehiclesLeft.VehicleSpawner` self _output_get_2))))

(fn `SpawnVehicleAtSpawnPoint`
  (`self.SpawnVehicle` (`SceneComponent.K2_GetComponentLocation` (`/Game/Blueprints/VehicleLaneSpawner.SpawnPoint` (`self.BP_Terrain`)))))

(fn `UserConstructionScript`)