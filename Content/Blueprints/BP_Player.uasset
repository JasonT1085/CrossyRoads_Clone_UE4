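; Player for a hop-based game in the Crossy Road style, with a score, HUD and level restart.
; Axis input, gated by a short cooldown and a trace for blockers, starts a fixed-step hop.
; Timelines arc the capsule to its target, turn the mesh toward the move and refill an idle timer.
; Tick counts that timer down, and on expiry input is disabled and BP_Eagle spawns once.
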(event `HopCooldown`
  (`/Engine/EditorBlueprintResources/StandardMacros.DoOnce` false :!label _label
    (:`Completed`
      (set `self.canHop` false)
      (`KismetSystemLibrary.Delay` 0.5)
      (set `self.canHop` true)
      (goto _label :!via `Reset`))))

(event `self.ReceiveTick`
  (params (DeltaSeconds :type "Float (single-precision)"))
  (set `self.EagleTimer` (- (`self.EagleTimer`) DeltaSeconds))
  (`self.Eagle Death`))

(event `Hop`
  (params (JumpVel :type "Float (double-precision)") (MoveRight :type "Float (double-precision)") (Scale :type "Float (double-precision)"))
  (bind (_initialloc_x _initialloc_y _initialloc_z) (`KismetMathLibrary.BreakVector` (`self.InitialLoc`)))
  (bind (_initialloc_x_2 _initialloc_y_2) (`KismetMathLibrary.BreakVector` (`self.InitialLoc`)))
  (bind (_finalloc_x _finalloc_y) (`KismetMathLibrary.BreakVector` (`self.FinalLoc`)))
  (bind _returnvalue (`SceneComponent.K2_GetComponentLocation` (`self.CapsuleComponent`)))
  (`GameplayStatics.PlaySound2D` "/Game/Sound/hop.hop" 1.0 1.0 0.0 null null)
  (set `self.InitialLoc` _returnvalue)
  (set `self.FinalLoc` (+ _returnvalue (`KismetMathLibrary.MakeVector` (* JumpVel Scale) (* MoveRight Scale))))
  (bind (_direction _movement _hop) (`Timeline|Timeline_0` :!via `PlayFromStart`)
    (:`Update`
      (bind _returnvalue_2 (`KismetMathLibrary.Lerp` _initialloc_z (+ _initialloc_z 55.0) _hop))
      (`SceneComponent.K2_SetWorldLocation` (`self.CapsuleComponent`) (`KismetMathLibrary.VLerp` (`KismetMathLibrary.MakeVector` _initialloc_x_2 _initialloc_y_2 _returnvalue_2) (`KismetMathLibrary.MakeVector` _finalloc_x _finalloc_y _returnvalue_2) _movement) false true))))

(event `Eagle Death`
  (if (<= (`self.EagleTimer`) 0.0)
    (`self.DisableInput` null)
    (`/Engine/EditorBlueprintResources/StandardMacros.DoOnce` false
      (:`Completed`
        (`|SpawnActorFromClass` "/Game/Blueprints/BP_Eagle.BP_Eagle_C" (`KismetMathLibrary.MakeTransform` (`SceneComponent.K2_GetComponentLocation` (`self.EagleSpawn`))) "Undefined" "OverrideRootScale" null null)))))

(event `InputAxis|Forward/Backward`
  (params (AxisValue :type "Float (single-precision)"))
  (bind _returnvalue (`self.K2_GetActorLocation`))
  (if (and (> (`KismetMathLibrary.Abs` AxisValue) 0.1) (`self.canHop`))
    (bind _outhit (`KismetSystemLibrary.BoxTraceSingle` _returnvalue (+ _returnvalue (* (`KismetMathLibrary.GetForwardVector` (`self.K2_GetActorRotation`)) (* AxisValue 100.0))) (10.0 10.0 10.0) (struct) "TraceTypeQuery1"))
    (if (not (`GameplayStatics.BreakHitResult` _outhit))
      (`self.HopCooldown`)
      (`self.Hop` AxisValue 0.0 80.0)
      (if (> AxisValue 0.3)
        (bind (_direction _rotation) (`Timeline|Timeline_1` :!via `PlayFromStart`)
          (:`Update`
            (`SceneComponent.K2_SetWorldRotation` (`self.StaticMesh`) (`KismetMathLibrary.RLerp` (`SceneComponent.K2_GetComponentRotation` (`self.StaticMesh`)) (struct :`Yaw` 180.0) _rotation true) false false)
            (set `self.EagleTimer` 15.0)))
        (else
          (bind (_direction_2 _rotation_2) (`Timeline|Timeline_2` :!via `PlayFromStart`)
            (:`Update`
              (`SceneComponent.K2_SetWorldRotation` (`self.StaticMesh`) (`KismetMathLibrary.RLerp` (`SceneComponent.K2_GetComponentRotation` (`self.StaticMesh`)) (struct) _rotation_2 true) false false)
              (set `self.EagleTimer` 15.0))))))))

(event `Restart`
  (bind _returnvalue (`GameplayStatics.GetCurrentLevelName` true))
  (`GameplayStatics.OpenLevel` (`KismetStringLibrary.Conv_StringToName` _returnvalue)))

(event `Add Score`
  (bind _result (`/Engine/EditorBlueprintResources/StandardMacros.IncrementFloat` (`self.Score`))
    (:`  `
      (set `self.Score` _result))))

(event `self.ReceiveBeginPlay`
  (bind _returnvalue (`|CreateWidget` "/Game/Blueprints/PlayerHUD.PlayerHUD_C"))
  (`UserWidget.AddToViewport` _returnvalue 0))

(event `InputAxis|Left/Right`
  (params (AxisValue :type "Float (single-precision)"))
  (bind _returnvalue (`self.K2_GetActorLocation`))
  (if (and (> (`KismetMathLibrary.Abs` AxisValue) 0.1) (`self.canHop`))
    (bind _outhit (`KismetSystemLibrary.SphereTraceSingle` _returnvalue (+ _returnvalue (* (`KismetMathLibrary.GetRightVector` (`self.K2_GetActorRotation`)) (* AxisValue 80.0))) 1.0 "TraceTypeQuery1"))
    (if (not (`GameplayStatics.BreakHitResult` _outhit))
      (`self.HopCooldown`)
      (`self.Hop` 0.0 AxisValue 80.0)
      (if (> 0.0 AxisValue)
        (bind (_direction _rotation) (`Timeline|Timeline_3` :!via `PlayFromStart`)
          (:`Update`
            (`SceneComponent.K2_SetWorldRotation` (`self.StaticMesh`) (`KismetMathLibrary.RLerp` (`SceneComponent.K2_GetComponentRotation` (`self.StaticMesh`)) (struct :`Yaw` 90.0) _rotation true) false false)
            (set `self.EagleTimer` 15.0)))
        (else
          (bind (_direction_2 _rotation_2) (`Timeline|Timeline_4` :!via `PlayFromStart`)
            (:`Update`
              (`SceneComponent.K2_SetWorldRotation` (`self.StaticMesh`) (`KismetMathLibrary.RLerp` (`SceneComponent.K2_GetComponentRotation` (`self.StaticMesh`)) (struct :`Yaw` 270.0) _rotation_2 true) false false)
              (set `self.EagleTimer` 15.0))))))))

(fn `UserConstructionScript`)