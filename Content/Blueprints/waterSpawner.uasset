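; Water lane hazard that spawns moving logs, kills the player on contact with its death zones and awards score once.
; BeginPlay randomly picks the lane's speed, side and looping spawn interval, negating projectile velocity for left-side logs.
; Two trigger zones destroy logs that reach them.
; Death and drown overlaps shrink the player's mesh to zero, play hurt and splash sounds, then reload the level after a delay.
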(event `self.ReceiveBeginPlay`
  (set `self.randomSpeed` (`KismetMathLibrary.RandomFloatInRange` 120.0 210.0))
  (set `self.SpawnLocation` (`SceneComponent.K2_GetComponentLocation` (`self.SpawnPoint`)))
  (set `self.SpawnLocationLeft` (`SceneComponent.K2_GetComponentLocation` (`self.SpawnpointLeft`)))
  (set `self.SetStartLocation` (`KismetMathLibrary.RandomBool`))
  (`KismetSystemLibrary.K2_SetTimerDelegate` (delegate `Spawn Logs`) (`KismetMathLibrary.RandomFloatInRange` 2.0 3.0) true))

(event `Spawn Logs`
  (if (`self.SetStartLocation`)
    (bind _returnvalue (`|SpawnActorFromClass` "/Game/Blueprints/Logs.Logs_C" (`KismetMathLibrary.MakeTransform` (`self.SpawnLocation`)) "Undefined" "OverrideRootScale" null null))
    (bind _projectilemovement (`/Game/Blueprints/Logs.ProjectileMovement` _returnvalue))
    (bind _output_get (set `ProjectileMovementComponent.InitialSpeed` (`self.randomSpeed`) _projectilemovement))
    (set `ProjectileMovementComponent.MaxSpeed` _output_get _projectilemovement)
    (else
      (bind _returnvalue_2 (`|SpawnActorFromClass` "/Game/Blueprints/Logs.Logs_C" (`KismetMathLibrary.MakeTransform` (`self.SpawnLocationLeft`)) "Undefined" "OverrideRootScale" null null))
      (bind _projectilemovement_2 (`/Game/Blueprints/Logs.ProjectileMovement` _returnvalue_2))
      (set `MovementComponent.Velocity` (`KismetMathLibrary.NegateVector` (`MovementComponent.Velocity` _projectilemovement_2)) _projectilemovement_2)
      (bind _projectilemovement_3 (`/Game/Blueprints/Logs.ProjectileMovement` _returnvalue_2))
      (bind _output_get_2 (set `ProjectileMovementComponent.InitialSpeed` (`self.randomSpeed`) _projectilemovement_3))
      (set `ProjectileMovementComponent.MaxSpeed` _output_get_2 _projectilemovement_3))))

(event `self.TriggerZone.OnComponentBeginOverlap`
  (params (OverlappedComponent :type "PrimitiveComponent Object Reference") (OtherActor :type "Actor Object Reference") (OtherComp :type "PrimitiveComponent Object Reference") (OtherBodyIndex :type Integer) (bFromSweep :type Boolean) (SweepResult :type "HitResult Structure (by ref)"))
  (bind _aslogs (cast `/Game/Blueprints/Logs` OtherActor))
  (`self.K2_DestroyActor` _aslogs))

(event `self.TriggerZone1.OnComponentBeginOverlap`
  (params (OverlappedComponent :type "PrimitiveComponent Object Reference") (OtherActor :type "Actor Object Reference") (OtherComp :type "PrimitiveComponent Object Reference") (OtherBodyIndex :type Integer) (bFromSweep :type Boolean) (SweepResult :type "HitResult Structure (by ref)"))
  (bind _aslogs (cast `/Game/Blueprints/Logs` OtherActor))
  (`self.K2_DestroyActor` _aslogs))

(event `OnPlayerDeath`
  (bind _returnvalue (`GameplayStatics.GetCurrentLevelName` true))
  (`GameplayStatics.OpenLevel` (`KismetStringLibrary.Conv_StringToName` _returnvalue)))

(event `self.DeathZone.OnComponentBeginOverlap`
  (params (OverlappedComponent :type "PrimitiveComponent Object Reference") (OtherActor :type "Actor Object Reference") (OtherComp :type "PrimitiveComponent Object Reference") (OtherBodyIndex :type Integer) (bFromSweep :type Boolean) (SweepResult :type "HitResult Structure (by ref)"))
  (bind _asbp_player (cast `/Game/Blueprints/BP_Player` OtherActor))
  (`SceneComponent.SetRelativeScale3D` (`/Game/Blueprints/BP_Player.StaticMesh` _asbp_player) (0.0 0.0 0.0))
  (`/Engine/EditorBlueprintResources/StandardMacros.DoOnce` false
    (:`Completed`
      (`GameplayStatics.PlaySound2D` "/Game/Sound/Chicken_hurt1.Chicken_hurt1" 1.0 1.0 0.0 null null)
      (`GameplayStatics.PlaySound2D` "/Game/Sound/352098__inspectorj__splash-jumping-d.352098__inspectorj__splash-jumping-d" 1.0 1.0 0.0 null null)
      (`KismetSystemLibrary.Delay` 2.0)
      (`self.OnPlayerDeath`))))

(event `self.DeathZone1.OnComponentBeginOverlap`
  (params (OverlappedComponent :type "PrimitiveComponent Object Reference") (OtherActor :type "Actor Object Reference") (OtherComp :type "PrimitiveComponent Object Reference") (OtherBodyIndex :type Integer) (bFromSweep :type Boolean) (SweepResult :type "HitResult Structure (by ref)"))
  (bind _asbp_player (cast `/Game/Blueprints/BP_Player` OtherActor))
  (`SceneComponent.SetRelativeScale3D` (`/Game/Blueprints/BP_Player.StaticMesh` _asbp_player) (0.0 0.0 0.0))
  (`/Engine/EditorBlueprintResources/StandardMacros.DoOnce` false
    (:`Completed`
      (`GameplayStatics.PlaySound2D` "/Game/Sound/Chicken_hurt1.Chicken_hurt1" 1.0 1.0 0.0 null null)
      (`GameplayStatics.PlaySound2D` "/Game/Sound/352098__inspectorj__splash-jumping-d.352098__inspectorj__splash-jumping-d" 1.0 1.0 0.0 null null)
      (`KismetSystemLibrary.Delay` 2.0)
      (`self.OnPlayerDeath`))))

(event `self.DrownCollision.OnComponentBeginOverlap`
  (params (OverlappedComponent :type "PrimitiveComponent Object Reference") (OtherActor :type "Actor Object Reference") (OtherComp :type "PrimitiveComponent Object Reference") (OtherBodyIndex :type Integer) (bFromSweep :type Boolean) (SweepResult :type "HitResult Structure (by ref)"))
  (bind _asbp_player (cast `/Game/Blueprints/BP_Player` OtherActor))
  (`SceneComponent.SetRelativeScale3D` (`/Game/Blueprints/BP_Player.StaticMesh` _asbp_player) (0.0 0.0 0.0))
  (`/Engine/EditorBlueprintResources/StandardMacros.DoOnce` false
    (:`Completed`
      (`GameplayStatics.PlaySound2D` "/Game/Sound/Chicken_hurt1.Chicken_hurt1" 1.0 1.0 0.0 null null)
      (`GameplayStatics.PlaySound2D` "/Game/Sound/352098__inspectorj__splash-jumping-d.352098__inspectorj__splash-jumping-d" 1.0 1.0 0.0 null null)
      (`KismetSystemLibrary.Delay` 2.0)
      (`self.OnPlayerDeath`))))

(event `self.ScoreCollision.OnComponentBeginOverlap`
  (params (OverlappedComponent :type "PrimitiveComponent Object Reference") (OtherActor :type "Actor Object Reference") (OtherComp :type "PrimitiveComponent Object Reference") (OtherBodyIndex :type Integer) (bFromSweep :type Boolean) (SweepResult :type "HitResult Structure (by ref)"))
  (bind _asbp_player (cast `/Game/Blueprints/BP_Player` OtherActor))
  (`/Engine/EditorBlueprintResources/StandardMacros.DoOnce` false
    (:`Completed`
      (`/Game/Blueprints/BP_Player.Add Score` _asbp_player))))

(fn `UserConstructionScript`)